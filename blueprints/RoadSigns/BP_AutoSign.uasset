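; Configurable road sign actor built from Pole, Front and Back components, with no active runtime logic.
; The construction script applies the Metal material to the pole.
; It creates separate dynamic instances of the existing Front and Back materials and feeds SignPng into the PNG texture parameter of both.
; One blueprint can thus show different sign images, with both faces sharing the same texture.
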(fn `UserConstructionScript`
  (bind _front (`self.Front`))
  (bind _back (`self.Back`))
  ;[1 1 1] Pole
  (`PrimitiveComponent.SetMaterial` (`self.Pole`) 0 (`self.Metal`))
  ;[1 1 1] Front
  (bind _returnvalue (`KismetMaterialLibrary.CreateDynamicMaterialInstance` (`PrimitiveComponent.GetMaterial` _front 0)))
  (`MaterialInstanceDynamic.SetTextureParameterValue` _returnvalue "PNG" (`self.Sign_png`))
  (`PrimitiveComponent.SetMaterial` _front 0 _returnvalue)
  ;[1 1 1] Back
  (bind _returnvalue_2 (`KismetMaterialLibrary.CreateDynamicMaterialInstance` (`PrimitiveComponent.GetMaterial` _back 0)))
  (`MaterialInstanceDynamic.SetTextureParameterValue` _returnvalue_2 "PNG" (`self.Sign_png`))
  (`PrimitiveComponent.SetMaterial` _back 0 _returnvalue_2))